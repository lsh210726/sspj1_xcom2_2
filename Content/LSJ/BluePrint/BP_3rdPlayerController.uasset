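; Player controller for an XCOM-style tactics game, handling player-turn input for moving and attacking.
; In move mode, one click spawns floor tiles from the character's reachable grid; the next walks the route and line-traces for cover.
; Attack mode checks the shot, plays a cinematic bullet burst, resolves hits through the GameState and ends the turn.
; Tab cycles characters or targets, Backspace ends character turns, and Delay loops drive movement and bullet timing.
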(event Custom|player%20turn%20tesk
  ;[1 1 1] PlayerTurnBegin
  (Development|PrintString "PlayerTurn")
  (Variables|Default|SetIsPlayerTurn true)
  (Variables|Default|SetPlayerActionModeSelection 0)
  ;;[1 1 1] get UI
  (bind _returnvalue (UserInterface|CreateWidget "/Game/LSJ/UI/WBP_PlayerActionUI.WBP_PlayerActionUI_C" (Game|GetPlayerController 0)))
  (Variables|Default|SetPlayer0ActionUI _returnvalue)
  (UserInterface|Viewport|AddtoViewport (Variables|Default|GetPlayer0ActionUI) 1000)
  (Variables|/Game/LSJ/UI/WBP_PlayerActionUI.WBP_PlayerActionUI_C|Set3rdPlayerController (Variables|Default|GetPlayer0ActionUI) self))

(event Custom|PlayerUIswitchAttack_Event
  ;[1 1 1] 1, 2 키 입력 shiftAction
  ;;[1 1 1] shiftAction Disable ::TODO
  (Variables|Default|SetPlayerActionModeSelection 1))

(event Custom|WhenComputingAccuacy_Event
  (bind _player0focusenemyui (Variables|Default|GetPlayer0FocusEnemyUI))
  (bind _asbp_cbase_actor (Utilities|Casting|CastToBP_CBaseActor (Variables|Default|GetAsSelectedBP_Enemy)))
  (bind _accuracy (CallFunction|ComputingAccuracy _asbp_cbase_actor (Variables|Default|GetAsSelectedBP_Player)))
  (Variables|/Game/LSJ/UI/WBP_PlayerFocusEnemy.WBP_PlayerFocusEnemy_C|Setaccuracy _player0focusenemyui _accuracy)
  (UserInterface|Viewport|AddtoViewport _player0focusenemyui 1000))

(event Custom|PlayerTurnBegin_Event)

(event Custom|PlayerActionPlayAttack_Event
  (bind _asselectedbp_player (Variables|Default|GetAsSelectedBP_Player))
  (bind _asselectedbp_enemy (Variables|Default|GetAsSelectedBP_Enemy))
  (bind _bp_camera (Variables|Default|GetBP_Camera))
  (bind _playerturnendsequance (Variables|Default|GetPlayerTurnEndSequance))
  (if (Variables|Default|GetIsAttackFinish)
    (|SetBy-RefVar (Variables|Default|GetIsAttackFinish) false)
    ;[1 1 1] UI off
    (Default|CallNewEventDispatcher (Variables|Default|GetPlayer0FocusEnemyUI))
    ;[1 1 1] 적 특정, 공격 가능한지 bool 출력
    (bind _intvector (Default|VectorLocation2IntLocation _asselectedbp_player (Transformation|GetActorLocation _asselectedbp_player)))
    (bind _intvector_2 (Default|VectorLocation2IntLocation _asselectedbp_player (Transformation|GetActorLocation _asselectedbp_enemy)))
    (bind (_couldattack _distance) (Default|SelectEnemy _asselectedbp_player _intvector _intvector_2 (Utilities|Array|MakeArray _asselectedbp_enemy)))
    (if _couldattack
      ;[1 1 1] 공격시 적을 바라보기
      (Default|RotateforLookActorDirection _asselectedbp_player _asselectedbp_enemy)
      ;[1 1 1] 총알 발사
      (Default|CinematicViewActor2Actor _bp_camera _asselectedbp_player _asselectedbp_enemy)
      (Variables|/Game/LSJ/BluePrint/ABP_Player.ABP_Player_C|SetEPlayerStatement (Variables|/Game/LSJ/BluePrint/BP_Player.BP_Player_C|GetAs%20ABP%20Player _asselectedbp_player) "NewEnumerator2")
      (Variables|Default|SetBulletCount 0)
      (bind _result (Math|Integer|IncrementInt (Variables|Default|GetBulletCount) :!label _label)
        (:%20%20
          (if (>= 6 _result)
            (bind (_outbullet _speed) (Default|Attack _asselectedbp_player (Variables|Default|GetBP_Bullet) _asselectedbp_enemy))
            (Actor|SetLifeSpan _outbullet (/ _distance _speed))
            (Utilities|FlowControl|Delay (Variables|Default|GetAttack_FireRate))
            (goto _label)
            (else
              (Variables|Default|SetBulletReachedCountTime 0.0)
              (Variables|Default|SetBulletReachedCountTime (+ (Variables|Default|GetBulletReachedCountTime) (Utilities|Time|GetWorldDeltaSeconds)) :!label _label_2)
              (bind _output_get (Variables|Default|SetIsReachedBullet (>= (* _speed (Variables|Default|GetBulletReachedCountTime)) _distance)))
              (if _output_get
                (bind _asbp_cbase_actor (Utilities|Casting|CastToBP_CBaseActor (Variables|Default|GetAsSelectedBP_Enemy))
                  (:then
                    (Default|ComputingHitEnemy (Variables|Default|GetAs%20BP%20XCOMGame%20State%20Base) _asbp_cbase_actor (Variables|Default|GetAsSelectedBP_Player))
                    ;[1 1 1] TODO:Animation Finish Delay
                    (Utilities|FlowControl|Delay 1.0)
                    (Default|ReturnPlayerCameraLocation _bp_camera)
                    (Variables|Default|SetIsAttackFinish true :!label _label_3)
                    (Variables|Default|SetIsPlayerTurn false)
                    (Default|SetPlayerTurnOff (Variables|Default|GetAs%20BP%20XCOMGame%20State%20Base))
                    ;[1 1 1] 초기화
                    (for (_ _array_index) _playerturnendsequance
                      (|SetBy-RefVar (Utilities|Array|Get(acopy) _playerturnendsequance _array_index) true)))
                  (:CastFailed
                    (Development|PrintString (Utilities|String|Append "BP_3rdPlayerController::" "Failed_" "Cast To " "CBaseActor"))))
                (else
                  (Utilities|FlowControl|Delay (Utilities|Time|GetWorldDeltaSeconds))
                  (goto _label_2)))))))
      (else
        (goto _label_3)))
    (else
      (Development|PrintString (Utilities|String|Append "BP_3rdPlayerController::" "Failed_" "CantAction" "_WhenAttackingActor")))))

(event EventBeginPlay
  (bind _returnvalue (Game|GetPlayerController 0))
  ;[1 1 1] 각 var와 Array에 Actor 대입
  ;;[1 1 1] UI
  (bind _returnvalue_2 (UserInterface|CreateWidget "/Game/LSJ/UI/WBP_PlayerActionUI.WBP_PlayerActionUI_C" _returnvalue))
  (Variables|Default|SetPlayer0ActionUI _returnvalue_2)
  (bind _returnvalue_3 (UserInterface|CreateWidget "/Game/LSJ/UI/WBP_PlayerFocusEnemy.WBP_PlayerFocusEnemy_C" _returnvalue))
  (Variables|Default|SetPlayer0FocusEnemyUI _returnvalue_3)
  (Utilities|Array|Clear (Variables|Default|GetEnemyTargets))
  (Utilities|Array|Clear (Variables|Default|GetPlayerTurnSequance))
  (bind _asbp_xcomgame_state_base (Utilities|Casting|CastToBP_XCOMGameStateBase (Game|GetGameState))
    (:then
      (bind _output_get (Variables|Default|SetAs%20BP%20XCOMGame%20State%20Base _asbp_xcomgame_state_base))
      (bind _outactors (Actor|GetAllActorsOfClass "/Game/LSJ/BluePrint/BP_Player.BP_Player_C"))
      ;;[1 1 1] Player,Enemy actors  Array에 입력, index0은 select
      (for (_array_element _array_index) _outactors
        (Utilities|Array|Add (Variables|Default|GetPlayerTurnSequance) _array_element)
        (Utilities|Array|Add (Variables|Default|GetPlayerTurnEndSequance) true)
        (if (== _array_index 0)
          (Variables|Default|SetAsSelectedBP_Player _array_element)))
      (bind _outactors_2 (Actor|GetAllActorsOfClass "/Game/Actor/CActor/BP_CBaseActor.BP_CBaseActor_C"))
      (for (_array_element_2 _array_index_2) _outactors_2
        (Utilities|Array|Add (Variables|Default|GetEnemyTargets) _array_element_2)
        (if (== _array_index_2 0)
          (Variables|Default|SetAsSelectedBP_Enemy _array_element_2)))
      (bind _returnvalue_4 (Actor|GetActorOfClass "/Game/LSJ/BluePrint/BP_CameraPawn.BP_CameraPawn_C"))
      (Variables|Default|SetBP_Camera _returnvalue_4)
      (bind _returnvalue_5 (Actor|GetActorOfClass "/Game/LSJ/BluePrint/BP_Bullet.BP_Bullet_C"))
      (Variables|Default|SetBP_Bullet _returnvalue_5)
      (bind _returnvalue_6 (Actor|GetActorOfClass "/Game/LSJ/BluePrint/BP_Floor.BP_Floor_C"))
      (Development|PrintString (Utilities|GetDisplayName _returnvalue_6))
      (Variables|Default|SetAsBP_Floor _returnvalue_6)
      (EventDispatchers|BindEventtoPlayerTurnDispatcher _output_get (delegate Custom|player%20turn%20tesk))
      (EventDispatchers|BindEventtoPlayerActionPlayAttack (delegate Custom|PlayerActionPlayAttack_Event))
      (EventDispatchers|BindEventtoPlayerUIswitchAttack (delegate Custom|PlayerUIswitchAttack_Event)))
    (:CastFailed
      (Development|PrintString (Utilities|String|Append "BP_3rdPlayerController::" "Failed_" "Cast To BP_XCOMGameStateBase")))))

(event EventTick
  (params (DeltaSeconds :type Float%20%28single-precision%29)))

(event Input|ActionEvents|InputActionBackspace
  (params (Key :type Key%20Structure :default "None"))
  (bind _selectedplayerindex (Variables|Default|GetSelectedPlayerIndex))
  (bind _playerturnendsequance (Variables|Default|GetPlayerTurnEndSequance))
  (bind _playerturnendsequance_2 (Variables|Default|GetPlayerTurnEndSequance))
  ;[1 1 1] Backspace
  (:Pressed
    ;[1 1 1] 캐릭터가 이동중인지 체크
    (if (Variables|Default|GetIsActorMoveFinish)
      ;[1 1 1] 플레이어 턴인지 체크
      (if (Variables|Default|GetIsPlayerTurn)
        ;[1 1 1] 캐릭터 턴 종료
        (Utilities|Array|SetArrayElem _playerturnendsequance _selectedplayerindex false)
        (bind _outnextplayerindex (CallFunction|PlayerCharTurnEndChecker _selectedplayerindex 0 _playerturnendsequance))
        (Variables|Default|SetAsSelectedBP_Player (Utilities|Array|Get(acopy) (Variables|Default|GetPlayerTurnSequance) _outnextplayerindex))
        (if (not (Utilities|Array|Get(acopy) _playerturnendsequance _outnextplayerindex))
          (if (not (Utilities|Array|ContainsItem _playerturnendsequance true))
            (Variables|Default|SetIsPlayerTurn false)
            (Default|SetPlayerTurnOff (Variables|Default|GetAs%20BP%20XCOMGame%20State%20Base))
            ;[1 1 1] 초기화
            (for (_ _array_index) _playerturnendsequance_2
              (|SetBy-RefVar (Utilities|Array|Get(acopy) _playerturnendsequance_2 _array_index) true))))
        (else
          (Development|PrintString (Utilities|String|Append "BP_3rdPlayerController::" "Failed_" "CantEndTurn" "_WhenIsntPlayerTurn"))))
      (else
        (Development|PrintString (Utilities|String|Append "BP_3rdPlayerController::" "Failed_" "CantEndTurnPlayerChar" "_WhenActorMoving"))))))

(event Input|ActionEvents|InputActionTab
  (params (Key :type Key%20Structure :default "None"))
  (bind _bp_camera (Variables|Default|GetBP_Camera))
  (bind _couldattackenemy (Variables|Default|GetCouldAttackEnemy))
  (bind _playerturnsequance (Variables|Default|GetPlayerTurnSequance))
  (bind _out_floor_actors (Variables|Default|GetOut%20Floor%20Actors))
  ;[1 1 1] tab
  (:Pressed
    ;[1 1 1] 캐릭터가 이동중인지 체크
    (if (Variables|Default|GetIsActorMoveFinish)
      ;[1 1 1] 플레이어 턴인지 체크
      (if (Variables|Default|GetIsPlayerTurn)
        (for _array_element _out_floor_actors
          (Actor|DestroyActor _array_element))
        (Utilities|Array|Clear _out_floor_actors)
        (|SetBy-RefVar (Variables|Default|GetTranslateCouldMakeTile) true)
        ;[1 1 1] shift Action
        (switch int (Variables|Default|GetPlayerActionModeSelection)
          (:0
            ;[1 1 1] 플레이어 선택
            (bind _outnextplayerindex (CallFunction|PlayerCharTurnEndChecker (Variables|Default|GetSelectedPlayerIndex) _playerturnsequance (Variables|Default|GetPlayerTurnEndSequance)))
            (bind _output_get (Variables|Default|SetAsSelectedBP_Player (Utilities|Array|Get(acopy) _playerturnsequance _outnextplayerindex)))
            (Development|PrintString (Utilities|GetDisplayName _output_get))
            ;[1 1 1] 카메라 포커싱
            (Default|CameraFocusActor _bp_camera (Variables|Default|GetAsSelectedBP_Player)))
          (:1
            ;[1 1 1] 공격 가능한 유닛 확인 TODO:
            (Utilities|Array|Clear _couldattackenemy)
            (for _array_element_2 (Variables|Default|GetEnemyTargets)
              ;[1 1 1] 적 특정, 공격 가능한지 bool 출력
              (bind _intvector (Default|VectorLocation2IntLocation (Variables|Default|GetAsSelectedBP_Player) (Transformation|GetActorLocation (Variables|Default|GetAsSelectedBP_Player))))
              (bind _intvector_2 (Default|VectorLocation2IntLocation (Variables|Default|GetAsSelectedBP_Player) (Transformation|GetActorLocation _array_element_2)))
              (bind _couldattack (Default|SelectEnemy (Variables|Default|GetAsSelectedBP_Player) _intvector _intvector_2 (Utilities|Array|MakeArray _array_element_2)))
              (Utilities|Array|Add _couldattackenemy _couldattack))
            ;[1 1 1] 적 선택
            (bind _outnextplayerindex_2 (CallFunction|EnemyCharSelectChecker (Variables|Default|GetSelectedEnemyIndex) _couldattackenemy))
            (bind _output_get_2 (Variables|Default|SetAsSelectedBP_Enemy (Utilities|Array|Get(acopy) (Variables|Default|GetEnemyTargets) _outnextplayerindex_2)))
            (Development|PrintString (Utilities|GetDisplayName _output_get_2))
            (Default|FocusActor2Actor _bp_camera (Variables|Default|GetAsSelectedBP_Player) (Variables|Default|GetAsSelectedBP_Enemy))))
        (else
          (Development|PrintString (Utilities|String|Append "BP_3rdPlayerController::" "Failed_" "CantShiftPlayer" "_WhenIsntPlayerTurn"))))
      (else
        (Development|PrintString (Utilities|String|Append "BP_3rdPlayerController::" "Failed_" "CantShiftPlayerChar" "_WhenActorMoving"))))))

(event Input|ActionEvents|InputActionOnClick
  (params (Key :type Key%20Structure :default "None"))
  (bind _asselectedbp_player (Variables|Default|GetAsSelectedBP_Player))
  (bind _asselectedbp_player_2 (Variables|Default|GetAsSelectedBP_Player))
  (bind _asselectedbp_enemy (Variables|Default|GetAsSelectedBP_Enemy))
  (bind _bp_camera (Variables|Default|GetBP_Camera))
  (bind _playerturnendsequance (Variables|Default|GetPlayerTurnEndSequance))
  (bind _addblocks (Variables|Default|GetaddBlocks))
  (bind _returnvalue (Transformation|GetActorLocation _asselectedbp_player))
  (bind _array (Utilities|Array|MakeArray _asselectedbp_player))
  (bind _routeresult (Variables|/Game/LSJ/BluePrint/BP_Player.BP_Player_C|GetRouteResult _asselectedbp_player))
  ;[1 1 1] click
  (:Pressed
    ;[1 1 1] 플레이어 턴인지 체크
    (if (Variables|Default|GetIsPlayerTurn)
      ;[1 1 1] switch 이동 0 공격 1
      (switch int (Variables|Default|GetPlayerActionModeSelection)
        (:0
          (if (Variables|Default|GetIsActorMoveFinish)
            (|SetBy-RefVar (Variables|Default|GetIsActorMoveFinish) false)
            (bind (_x _y) (CallFunction|GettoPoint self))
            (Variables|/Game/LSJ/BluePrint/BP_Player.BP_Player_C|SetFind%20Location _asselectedbp_player (Utilities|Struct|MakeIntVector _x _y))
            (if (Variables|Default|GetTranslateCouldMakeTile)
              (Utilities|Array|Clear _addblocks)
              (Utilities|Array|AppendArray _addblocks (Variables|Default|GetPlayerTurnSequance))
              ;[1 1 1] 이동
              (Utilities|Array|AppendArray _addblocks (Variables|Default|GetEnemyTargets))
              ;;[1 1 1] 이동 가능한 위치 생성
              (Default|SetMoveLocation _asselectedbp_player true _addblocks)
              ;;[1 1 1] 바닥에 이동 가능 위치 장판깔기
              (bind _keys (Utilities|Map|Keys (Variables|/Game/LSJ/BluePrint/BP_Player.BP_Player_C|GetGreedy%20Map _asselectedbp_player)))
              (bind _outflooractors (CallFunction|MakePlayerMoveDistanceFloor _asselectedbp_player (Variables|Default|GetAsBP_Floor) _keys))
              (|SetBy-RefVar (Variables|Default|GetTranslateCouldMakeTile) false)
              (|SetBy-RefVar (Variables|Default|GetIsActorMoveFinish) true)
              (Variables|Default|SetOut%20Floor%20Actors _outflooractors)
              (else
                (|SetBy-RefVar (Variables|Default|GetTranslateCouldMakeTile) true)
                (for _array_element (Variables|Default|GetOut%20Floor%20Actors)
                  (Actor|DestroyActor _array_element))
                (Utilities|Array|Clear (Variables|Default|GetOut%20Floor%20Actors))
                (Variables|Default|SetCover 20)
                (Default|GetMoveLocation _asselectedbp_player)
                (|SetBy-RefVar (Variables|Default|GetTranslateRouteResultIteration))
                (Variables|/Game/LSJ/BluePrint/ABP_Player.ABP_Player_C|SetEPlayerStatement (Variables|/Game/LSJ/BluePrint/BP_Player.BP_Player_C|GetAs%20ABP%20Player _asselectedbp_player) "NewEnumerator0")
                (if (or (and (>= (Variables|Default|GetTranslateRouteResultIteration) (Utilities|Array|Length _routeresult)) (Variables|Default|GetIsTranslateFinish)) (Variables|Default|GetIsTranslateFinish)) :!label _label
                  (Variables|Default|SetIsTranslateFinish false)
                  (bind _result (Math|Integer|IncrementInt (Variables|Default|GetTranslateRouteResultIteration))
                    (:%20%20
                      (Variables|Default|SetTranslateRouteResultIteration _result))))
                (if (>= (Variables|Default|GetTranslateRouteResultIteration) (Utilities|Array|Length _routeresult))
                  (Variables|/Game/LSJ/BluePrint/BP_Player.BP_Player_C|SetIsNeedMakeGreedMap _asselectedbp_player true)
                  (Variables|Default|SetIsActorMoveFinish true)
                  ;[1 1 1] cover
                  (bind _outhit (Collision|LineTraceByChannel _returnvalue (+ _returnvalue "100.000000,0.000000,0.000000") "TraceTypeQuery1" false _array "ForDuration"))
                  (bind _outhit_2 (Collision|LineTraceByChannel _returnvalue (+ _returnvalue "-100.000000,0.000000,0.000000") "TraceTypeQuery1" false _array "ForDuration"))
                  (bind _outhit_3 (Collision|LineTraceByChannel _returnvalue (+ _returnvalue "0.000000,-100.000000,0.000000") "TraceTypeQuery1" false _array "ForDuration"))
                  (bind _outhit_4 (Collision|LineTraceByChannel _returnvalue (+ _returnvalue "0.000000,100.000000,0.000000") "TraceTypeQuery1" false _array "ForDuration"))
                  (if (Math|Boolean|ORBoolean (.bblockinghit _outhit) (.bblockinghit _outhit_2) (.bblockinghit _outhit_3) (.bblockinghit _outhit_4))
                    (Variables|Default|SetCover 40)
                    ;[1 1 1] Comment
                    (Variables|/Game/LSJ/BluePrint/ABP_Player.ABP_Player_C|SetEPlayerStatement (Variables|/Game/LSJ/BluePrint/BP_Player.BP_Player_C|GetAs%20ABP%20Player _asselectedbp_player) "NewEnumerator1")
                    (else
                      (Variables|Default|SetCover 0)
                      (Variables|/Game/LSJ/BluePrint/ABP_Player.ABP_Player_C|SetEPlayerStatement (Variables|/Game/LSJ/BluePrint/BP_Player.BP_Player_C|GetAs%20ABP%20Player _asselectedbp_player) "NewEnumerator5")))
                  (else
                    (bind _isfinish (Default|Translate _asselectedbp_player (.X (Utilities|Struct|BreakIntVector (Utilities|Array|Get(acopy) _routeresult (Variables|Default|GetTranslateRouteResultIteration)))) (.Y (Utilities|Struct|BreakIntVector (Utilities|Array|Get(acopy) _routeresult (Variables|Default|GetTranslateRouteResultIteration))))))
                    (Variables|Default|SetIsTranslateFinish _isfinish)
                    (Utilities|FlowControl|Delay (Utilities|Time|GetWorldDeltaSeconds))
                    (goto _label)))))
            (else
              (Development|PrintString (Utilities|String|Append "BP_3rdPlayerController::" "Failed_" "CantMovePlayer" "_WhenActorMoving")))))
        (:1
          (if (Variables|Default|GetIsAttackFinish)
            (|SetBy-RefVar (Variables|Default|GetIsAttackFinish) false)
            ;[1 1 1] UI off
            (Default|CallNewEventDispatcher (Variables|Default|GetPlayer0FocusEnemyUI))
            ;[1 1 1] 적 특정, 공격 가능한지 bool 출력
            (bind _intvector (Default|VectorLocation2IntLocation _asselectedbp_player_2 (Transformation|GetActorLocation _asselectedbp_player_2)))
            (bind _intvector_2 (Default|VectorLocation2IntLocation _asselectedbp_player_2 (Transformation|GetActorLocation _asselectedbp_enemy)))
            (bind (_couldattack _distance) (Default|SelectEnemy _asselectedbp_player_2 _intvector _intvector_2 (Utilities|Array|MakeArray _asselectedbp_enemy)))
            (if _couldattack
              ;[1 1 1] 공격시 적을 바라보기
              (Default|RotateforLookActorDirection _asselectedbp_player_2 _asselectedbp_enemy)
              ;[1 1 1] 총알 발사
              (Default|CinematicViewActor2Actor _bp_camera _asselectedbp_player_2 _asselectedbp_enemy)
              (Variables|/Game/LSJ/BluePrint/ABP_Player.ABP_Player_C|SetEPlayerStatement (Variables|/Game/LSJ/BluePrint/BP_Player.BP_Player_C|GetAs%20ABP%20Player _asselectedbp_player_2) "NewEnumerator2")
              (Variables|Default|SetBulletCount 0)
              (bind _result_2 (Math|Integer|IncrementInt (Variables|Default|GetBulletCount) :!label _label_2)
                (:%20%20
                  (if (>= 6 _result_2)
                    (bind (_outbullet _speed) (Default|Attack _asselectedbp_player_2 (Variables|Default|GetBP_Bullet) _asselectedbp_enemy))
                    (Actor|SetLifeSpan _outbullet (/ _distance _speed))
                    (Utilities|FlowControl|Delay (Variables|Default|GetAttack_FireRate))
                    (goto _label_2)
                    (else
                      (Variables|Default|SetBulletReachedCountTime 0.0)
                      (Variables|Default|SetBulletReachedCountTime (+ (Variables|Default|GetBulletReachedCountTime) (Utilities|Time|GetWorldDeltaSeconds)) :!label _label_3)
                      (bind _output_get (Variables|Default|SetIsReachedBullet (>= (* _speed (Variables|Default|GetBulletReachedCountTime)) _distance)))
                      (if _output_get
                        (bind _asbp_cbase_actor (Utilities|Casting|CastToBP_CBaseActor (Variables|Default|GetAsSelectedBP_Enemy))
                          (:then
                            (Default|ComputingHitEnemy (Variables|Default|GetAs%20BP%20XCOMGame%20State%20Base) _asbp_cbase_actor (Variables|Default|GetAsSelectedBP_Player))
                            ;[1 1 1] TODO:Animation Finish Delay
                            (Utilities|FlowControl|Delay 1.0)
                            (Default|ReturnPlayerCameraLocation _bp_camera)
                            (Variables|Default|SetIsAttackFinish true :!label _label_4)
                            (Variables|Default|SetIsPlayerTurn false)
                            (Default|SetPlayerTurnOff (Variables|Default|GetAs%20BP%20XCOMGame%20State%20Base))
                            ;[1 1 1] 초기화
                            (for (_ _array_index) _playerturnendsequance
                              (|SetBy-RefVar (Utilities|Array|Get(acopy) _playerturnendsequance _array_index) true)))
                          (:CastFailed
                            (Development|PrintString (Utilities|String|Append "BP_3rdPlayerController::" "Failed_" "Cast To " "CBaseActor"))))
                        (else
                          (Utilities|FlowControl|Delay (Utilities|Time|GetWorldDeltaSeconds))
                          (goto _label_3)))))))
              (else
                (goto _label_4)))
            (else
              (Development|PrintString (Utilities|String|Append "BP_3rdPlayerController::" "Failed_" "CantAction" "_WhenAttackingActor"))))))
      (else
        (Development|PrintString (Utilities|String|Append "BP_3rdPlayerController::" "Failed_" "CantAction" "_WhenIsntPlayerTurn"))))))

(event Input|KeyboardEvents|1
  (params (Key :type Key%20Structure :default "None"))
  ;[1 1 1] 1, 2 키 입력 shiftAction
  (:Pressed
    (Development|PrintString (Utilities|String|Append "MoveMode" " LMB: " "Move" " TAB: " "ShiftPlayerCharactor"))
    (Variables|Default|SetPlayerActionModeSelection 0)))

(event Input|KeyboardEvents|2
  (params (Key :type Key%20Structure :default "None"))
  ;[1 1 1] 1, 2 키 입력 shiftAction
  (:Pressed
    (Development|PrintString (Utilities|String|Append "AttackMode" " LMB: " "Attack" " TAB: " "ShiftEnemyCharactor"))
    ;;[1 1 1] shiftAction Disable ::TODO
    (Default|CallOnReleasedAttackCustom (Variables|Default|GetPlayer0ActionUI))
    (Variables|Default|SetPlayerActionModeSelection 1)))

(fn ConstructionScript)

(fn GettoPoint
  (bind _hitresult (Game|Player|GetHitResultUnderCursorbyChannel "TraceTypeQuery1" false))
  (bind (_x _y) (Math|Vector|BreakVector (.location _hitresult)))
  (bind _returnvalue (* _x 0.01))
  (bind _returnvalue_2 (* _y 0.01))
  (bind _returnvalue_3 (Math|Float|Floor _returnvalue_2))
  (bind _returnvalue_4 (Math|Float|Floor _returnvalue))
  (Development|PrintString (Utilities|String|Append "MousePointer: (" (Utilities|String|ToString(Integer) _returnvalue_4) ", " (Utilities|String|ToString(Integer) _returnvalue_3) ")") true true "(R=0.000000,G=0.660000,B=1.000000,A=1.000000)" 0.1 "")
  (return _returnvalue_4 _returnvalue_3))

(fn TurnManager
  (params (InPlayer :type Array%20of%20Actor%20Object%20References) (NewParam1 :type Integer))
  (return))

(fn PlayerCharTurnEndChecker
  (params (InPlayerIndex :type Integer%20%28by%20ref%29) (PlayerTurnSequance :type Array%20of%20BP%20Player%20Object%20References) (hasPlayerCharTurn :type Array%20of%20Booleans))
  (Math|Integer|IncrementInt InPlayerIndex :!label _label
    (:%20%20
      (if (Utilities|Array|IsValidIndex hasPlayerCharTurn InPlayerIndex)
        (if (Utilities|Array|Get(acopy) hasPlayerCharTurn InPlayerIndex)
          _
          (else
            (goto _label)))
        (else
          (|SetBy-RefVar InPlayerIndex)))
      (return InPlayerIndex))))

(fn EnemyCharSelectChecker
  (params (InSelectedEnemyIndex :type Integer%20%28by%20ref%29) (CouldAttack :type Array%20of%20Booleans))
  (Math|Integer|IncrementInt InSelectedEnemyIndex :!label _label
    (:%20%20
      (if (Utilities|Array|IsValidIndex CouldAttack InSelectedEnemyIndex)
        (if (Utilities|Array|Get(acopy) CouldAttack InSelectedEnemyIndex)
          _
          (else
            (goto _label)))
        (else
          (|SetBy-RefVar InSelectedEnemyIndex)))
      (return InSelectedEnemyIndex))))

(fn MakePlayerMoveDistanceFloor
  (params (SelctedPlayerChar :type Actor%20Object%20Reference%20%28by%20ref%29) (CopyFloorInstance :type Actor%20Object%20Reference%20%28by%20ref%29) (InPlayerMovableArea :type Array%20of%20Int%20Vector%20Structures))
  (bind _newlocalvar (LocalVariables|GetNewLocalVar))
  (for _array_element InPlayerMovableArea
    (bind _returnvalue (Game|SpawnActorfromClass (Utilities|GetClass CopyFloorInstance) (Math|Transform|MakeTransform (+ (* (Math|Conversions|ToVector(Float) _array_element) "100.000000,100.000000,0.000000") "50.000000,50.000000,0.100000") "0, 0, 0" "1.000000,1.000000,1.000000") "AlwaysSpawn" "MultiplyWithRoot" 0 0))
    (Rendering|SetActorHiddenInGame _returnvalue false)
    (Utilities|Array|Add _newlocalvar _returnvalue))
  (return _newlocalvar))

(fn ComputingAccuracy
  (params (Enemy :type BP%20C%20Base%20Actor%20Object%20Reference) (Player :type BP%20Player%20Object%20Reference))
  (return (+ (Variables|/Game/LSJ/BluePrint/BP_Player.BP_Player_C|GetDefaultAccuracy Player) (* (Variables|/Game/Actor/CActor/BP_CBaseActor.BP_CBaseActor_C|GetCover Enemy) -20)) (Variables|/Game/LSJ/BluePrint/BP_Player.BP_Player_C|GetDefaultDamage Player)))