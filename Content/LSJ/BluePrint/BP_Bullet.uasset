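; BP_Bullet is a simple projectile actor that flies in a straight line along its forward vector.
; Tick moves it each frame by Speed scaled by delta time, using SetActorLocation without sweep.
; The Cube component's begin-overlap event destroys the bullet when the other actor matches BP_CBaseActor, with no damage or other hit effect applied here.
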(event OnComponentBeginOverlap(Cube)
  (params (OverlappedComponent :type Primitive%20Component%20Object%20Reference) (OtherActor :type Actor%20Object%20Reference) (OtherComp :type Primitive%20Component%20Object%20Reference) (OtherBodyIndex :type Integer) (bFromSweep :type Boolean) (SweepResult :type Hit%20Result%20Structure%20%28by%20ref%29))
  (if (== OtherActor "/Game/Actor/CActor/BP_CBaseActor.BP_CBaseActor")
    (Actor|DestroyActor)))

(event EventBeginPlay)

(event Collision|EventActorBeginOverlap
  (params (OtherActor :type Actor%20Object%20Reference)))

(event EventTick
  (params (DeltaSeconds :type Float%20%28single-precision%29))
  (Transformation|SetActorLocation (+ (Transformation|GetActorLocation) (* (Math|Vector|Normalize (Transformation|GetActorForwardVector)) (Variables|Default|GetSpeed) DeltaSeconds)) false false))

(fn ConstructionScript)