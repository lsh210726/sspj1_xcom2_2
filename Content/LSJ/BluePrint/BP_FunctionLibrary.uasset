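; BP_FunctionLibrary is an Actor-style Blueprint holding helpers that convert between world positions and integer grid cells of 100 units.
; IntLocation2VectorLocation returns the XY center of a cell at Z zero.
; VectorLocation2IntLocation floors scaled X and Y into a cell with Z zero, but takes no input here and operates on constant zeros.
; The event graph and construction script do nothing.
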(event EventBeginPlay)

(event Collision|EventActorBeginOverlap
  (params (OtherActor :type Actor%20Object%20Reference)))

(event EventTick
  (params (DeltaSeconds :type Float%20%28single-precision%29)))

(fn ConstructionScript)

(fn VectorLocation2IntLocation
  (params (Vector :type Vector))
  (return (Utilities|Struct|MakeIntVector (Math|Float|Floor (* 0.0 0.01)) (Math|Float|Floor (* 0.0 0.01)))))

(fn IntLocation2VectorLocation
  (params (IntVector :type Int%20Vector%20Structure))
  (bind (_x _y) (Utilities|Struct|BreakIntVector IntVector))
  (return (Math|Vector|MakeVector (+ (* _x 1e+02) 5e+01) (+ (* _y 1e+02) 5e+01) 0.0)))