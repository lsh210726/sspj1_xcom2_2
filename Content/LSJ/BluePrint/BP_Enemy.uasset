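; BP_Enemy is an enemy Blueprint with grid movement and pathfinding helpers; Tick, CheckRoute8 and AttackRange are empty.
; Translate steps toward a 100-unit cell's center, returning true within 5 units and printing debug text labeled BP_Player.
; CheckRoute4 performs one breadth-first expansion over unblocked neighbors, storing parent and depth in GreedyMap and returning the next frontier.
; It computes a target-found flag but always returns false for it.
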(event EventTick
  (params (DeltaSeconds :type Float%20%28single-precision%29)))

(fn ConstructionScript)

(fn Translate
  (params (GetToPointX :type Integer) (GetToPointY :type Integer))
  (bind _returnvalue (Transformation|GetActorLocation))
  (bind _returnvalue_2 (Transformation|GetActorLocation))
  (bind _returnvalue_3 (Transformation|GetActorLocation))
  (bind _returnvalue_4 (Transformation|GetActorLocation))
  (bind _returnvalue_5 (Math|Float|Floor (.x _returnvalue_4)))
  (LocalVariables|SetPointX (+ (* GetToPointX 100) 50))
  (LocalVariables|SetPointY (+ (* GetToPointY 100) 50))
  (Transformation|SetActorLocation (+ (Transformation|GetActorLocation) (* (Math|Vector|Normalize (- (Math|Vector|MakeVector (Math|Conversions|ToFloat(Integer) (LocalVariables|GetPointX)) (Math|Conversions|ToFloat(Integer) (LocalVariables|GetPointY)) 0.0) (Math|Vector|MakeVector (.x _returnvalue_2) (.y _returnvalue_2) 0.0))) (Variables|Default|GetSpeed) (Utilities|Time|GetWorldDeltaSeconds))) false false)
  (if (>= (LocalVariables|GetPointX) 0)
    (LocalVariables|SetIsFinishX (and (<= (+ (LocalVariables|GetPointX) -5) _returnvalue_5) (<= _returnvalue_5 (+ (LocalVariables|GetPointX) 5))))
    (else
      (LocalVariables|SetIsFinishX (and (<= _returnvalue_5 (+ (LocalVariables|GetPointX) 5)) (<= (+ (LocalVariables|GetPointX) -5) _returnvalue_5)))))
  (if (>= (LocalVariables|GetPointY) 0)
    (LocalVariables|SetIsFinishY (and (<= (+ (LocalVariables|GetPointY) -5) (.y _returnvalue)) (<= (.y _returnvalue) (+ (LocalVariables|GetPointY) 5))))
    (else
      (LocalVariables|SetIsFinishY (and (<= (.y _returnvalue) (+ (LocalVariables|GetPointY) 5)) (<= (+ (LocalVariables|GetPointY) -5) (.y _returnvalue))))))
  (if (and (LocalVariables|GetIsFinishX) (LocalVariables|GetIsFinishY))
    (Development|PrintString (Utilities|String|Append "BP_Player Translate [ IsFinish(Location:" (Utilities|String|ToString(Float) (.x _returnvalue_3)) ", " (Utilities|String|ToString(Float) (.y _returnvalue_3)) "),  (Point:" (Utilities|String|ToString(Integer) (LocalVariables|GetPointX)) ", " (Utilities|String|ToString(Integer) (LocalVariables|GetPointY)) ")" ", (IsFinish X:" (Utilities|String|ToString(Boolean) (LocalVariables|GetIsFinishX)) ",  IsFinish Y:" (Utilities|String|ToString(Boolean) (LocalVariables|GetIsFinishY)) ") ]") true true "(R=0.000000,G=0.660000,B=1.000000,A=1.000000)" 5.0)
    (return (and (LocalVariables|GetIsFinishX) (LocalVariables|GetIsFinishY)))
    (else
      (Development|PrintString (Utilities|String|Append "BP_Player Translate [ IsFinish(Location:" (Utilities|String|ToString(Float) (.x _returnvalue_3)) ", " (Utilities|String|ToString(Float) (.y _returnvalue_3)) "),  (Point:" (Utilities|String|ToString(Integer) (LocalVariables|GetPointX)) ", " (Utilities|String|ToString(Integer) (LocalVariables|GetPointY)) ")" ", (IsFinish X:" (Utilities|String|ToString(Boolean) (LocalVariables|GetIsFinishX)) ",  IsFinish Y:" (Utilities|String|ToString(Boolean) (LocalVariables|GetIsFinishY)) ") ]") true true "(R=0.000000,G=0.660000,B=1.000000,A=1.000000)" (Utilities|Time|GetWorldDeltaSeconds))
      (return (and (LocalVariables|GetIsFinishX) (LocalVariables|GetIsFinishY))))))

(fn CheckRoute4
  (params (InGreedyMap :type Map%20of%20Int%20Vector%20Structures%20to%20Structs) (InBlockInfoMap :type Map%20of%20Int%20Vector%20Structures%20to%20Booleans) (InThisLocation :type Int%20Vector%20Structure) (InFindLocation :type Int%20Vector%20Structure) (InNowIteration :type Integer) (InMaxIteration :type Integer))
  (bind (_x _y) (Utilities|Struct|BreakIntVector InThisLocation))
  (bind (_x_2 _y_2) (Utilities|Struct|BreakIntVector InThisLocation))
  (bind (_x_3 _y_3) (Utilities|Struct|BreakIntVector InFindLocation))
  (bind (_x_4 _y_4) (Utilities|Struct|BreakIntVector InThisLocation))
  (bind (_x_5 _y_5) (Utilities|Struct|BreakIntVector InFindLocation))
  (bind (_x_6 _y_6) (Utilities|Struct|BreakIntVector InThisLocation))
  (bind (_x_7 _y_7) (Utilities|Struct|BreakIntVector InFindLocation))
  (bind (_x_8 _y_8) (Utilities|Struct|BreakIntVector InThisLocation))
  (bind (_x_9 _y_9) (Utilities|Struct|BreakIntVector InFindLocation))
  (bind (_x_10 _y_10) (Utilities|Struct|BreakIntVector InThisLocation))
  (bind (_x_11 _y_11) (Utilities|Struct|BreakIntVector InThisLocation))
  (bind (_x_12 _y_12) (Utilities|Struct|BreakIntVector InThisLocation))
  (bind _returnvalue (+ InNowIteration 1))
  (bind _returnvalue_2 (+ InNowIteration 1))
  (bind _returnvalue_3 (+ InNowIteration 1))
  (bind _returnvalue_4 (+ InNowIteration 1))
  (bind _returnvalue_5 (+ _y_11 -1))
  (bind _returnvalue_6 (+ _x 1))
  (bind _returnvalue_7 (+ _y_2 1))
  (bind _returnvalue_8 (+ _x_10 -1))
  (bind _intvector (Utilities|Struct|MakeIntVector _returnvalue_6 _y))
  (bind _intvector_2 (Utilities|Struct|MakeIntVector _x_2 _returnvalue_7))
  (bind _intvector_3 (Utilities|Struct|MakeIntVector _returnvalue_8 _y_10))
  (bind _intvector_4 (Utilities|Struct|MakeIntVector _x_11 _returnvalue_5))
  (LocalVariables|SetLocalNextLoopFindLocation (Utilities|Array|MakeArray))
  (Variables|Default|SetBlock%20Info%20Map InBlockInfoMap)
  (LocalVariables|SetLocalMaxIteration InMaxIteration)
  (LocalVariables|SetLocalIsFindMoveRoute false)
  (Utilities|FlowControl|Sequence
    (:then_0
      (if (>= (LocalVariables|GetLocalMaxIteration) InNowIteration)
        (if (not (.ReturnValue (Utilities|Map|Find (Variables|Default|GetGreedy%20Map) _intvector)))
          (if (not (.ReturnValue (Utilities|Map|Find (Variables|Default|GetBlock%20Info%20Map) _intvector)))
            (Utilities|Map|Add (Variables|Default|GetGreedy%20Map) _intvector (Utilities|Struct|MakeIntVector _x_4 _y_4 _returnvalue_2))
            (Utilities|Array|AppendArray (LocalVariables|GetLocalNextLoopFindLocation) (Utilities|Array|MakeArray (Utilities|Struct|MakeIntVector _returnvalue_6 _y _returnvalue_2)))
            (LocalVariables|SetLocalIsFindMoveRoute (and (== _returnvalue_6 _x_5) (== _y _y_5)))))
        (else
          (return (LocalVariables|GetLocalNextLoopFindLocation) true false))))
    (:then_1
      (if (>= (LocalVariables|GetLocalMaxIteration) InNowIteration)
        (if (not (.ReturnValue (Utilities|Map|Find (Variables|Default|GetGreedy%20Map) _intvector_2)))
          (if (not (.ReturnValue (Utilities|Map|Find (Variables|Default|GetBlock%20Info%20Map) _intvector_2)))
            (Utilities|Map|Add (Variables|Default|GetGreedy%20Map) _intvector_2 (Utilities|Struct|MakeIntVector _x_6 _y_6 _returnvalue_3))
            (Utilities|Array|AppendArray (LocalVariables|GetLocalNextLoopFindLocation) (Utilities|Array|MakeArray (Utilities|Struct|MakeIntVector _x_2 _returnvalue_7 _returnvalue_3)))
            (LocalVariables|SetLocalIsFindMoveRoute (or (LocalVariables|GetLocalIsFindMoveRoute) (and (== _x_2 _x_7) (== _returnvalue_7 _y_7))))))
        (else
          (return (LocalVariables|GetLocalNextLoopFindLocation) true false))))
    (:then_2
      (if (>= (LocalVariables|GetLocalMaxIteration) InNowIteration)
        (if (not (Utilities|Map|Contains (Variables|Default|GetGreedy%20Map) _intvector_3))
          (if (not (.ReturnValue (Utilities|Map|Find (Variables|Default|GetBlock%20Info%20Map) _intvector_3)))
            (Utilities|Map|Add (Variables|Default|GetGreedy%20Map) _intvector_3 (Utilities|Struct|MakeIntVector _x_8 _y_8 _returnvalue_4))
            (Utilities|Array|AppendArray (LocalVariables|GetLocalNextLoopFindLocation) (Utilities|Array|MakeArray (Utilities|Struct|MakeIntVector _returnvalue_8 _y_10 _returnvalue_4)))
            (LocalVariables|SetLocalIsFindMoveRoute (or (LocalVariables|GetLocalIsFindMoveRoute) (and (== _returnvalue_8 _x_9) (== _y_10 _y_9))))))
        (else
          (return (LocalVariables|GetLocalNextLoopFindLocation) true false))))
    (:then_3
      (if (>= (LocalVariables|GetLocalMaxIteration) InNowIteration)
        (if (not (.ReturnValue (Utilities|Map|Find (Variables|Default|GetGreedy%20Map) _intvector_4)))
          (if (not (.ReturnValue (Utilities|Map|Find (Variables|Default|GetBlock%20Info%20Map) _intvector_4)))
            (Utilities|Map|Add (Variables|Default|GetGreedy%20Map) _intvector_4 (Utilities|Struct|MakeIntVector _x_12 _y_12 _returnvalue))
            (Utilities|Array|AppendArray (LocalVariables|GetLocalNextLoopFindLocation) (Utilities|Array|MakeArray (Utilities|Struct|MakeIntVector _x_11 _returnvalue_5 _returnvalue)))
            (LocalVariables|SetLocalIsFindMoveRoute (or (LocalVariables|GetLocalIsFindMoveRoute) (and (== _x_11 _x_3) (== _returnvalue_5 _y_3))))))
        (return (LocalVariables|GetLocalNextLoopFindLocation) false false)
        (else
          (return (LocalVariables|GetLocalNextLoopFindLocation) true false))))))

(fn CheckRoute8)

(fn AttackRange)