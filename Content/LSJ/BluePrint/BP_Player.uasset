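; Player unit for grid-based movement and shooting on 100-unit cells.
; setMoveLocation marks blocked cells, then runs a four-way breadth-first search up to MaxIteration, storing parent cells in GreedyMap and backtracking from FindLocation into RouteResult.
; Translate steps and turns the actor toward a cell centre, reporting arrival.
; SelectEnemy line-traces for clear shots, Attack spawns a BP_Bullet facing the target, and AttackFocus points BP_CameraPawn at a given actor.
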(event Custom|getMoveLocation
  (bind _output_get (Variables|Default|SetIsNeedMakeGreedMap (stale Custom|setMoveLocation InputIsNeedMakeGreedMap)))
  (if _output_get
    (if (Variables|Default|GetIsMoveFinished)
      (bind _intvector (CallFunction|VectorLocation2IntLocation (Transformation|GetActorLocation)))
      (Variables|Default|SetPlayerLocation _intvector)
      ;[1 1 1] reset 0
      (Utilities|Array|Clear (Variables|Default|GetRouteResult))
      (Utilities|Array|Clear (Variables|Default|GetRouteTaskManager))
      (Utilities|Map|Clear (Variables|Default|GetGreedy%20Map))
      (Variables|Default|SetNowTesk 0)
      (Variables|Default|SetRouteTaskManager (Utilities|Array|MakeArray _intvector))
      ;[1 1 1] \GreedyMap에PlayerLocation부터 MaxIteration의 거리까지의 정보 f(x) = MI - pL * dt/dx를 이동한 경로값 (n+1,m),(n,m+1),(n-1,m),(n,m-1)의 Key, (n,m,Iteration)의 Value 형태를 Map으로 저장
      (for _index (range 0 (Variables|Default|GetMax%20Iteration))
        (while (== (.Z (Utilities|Struct|BreakIntVector (Utilities|Array|Get(acopy) (Variables|Default|GetRouteTaskManager) (Variables|Default|GetNowTesk)))) _index)
          (bind (_outnextlocations _outismaxiterationover _outisfindmoveroute) (CallFunction|CheckRoute4 (Variables|Default|GetGreedy%20Map) (Variables|Default|GetCalcBlockInfoMap) (Utilities|Array|Get(acopy) (Variables|Default|GetRouteTaskManager) (Variables|Default|GetNowTesk)) (Variables|Default|GetFind%20Location) _index (Variables|Default|GetMax%20Iteration)))
          (if (not _outismaxiterationover)
            (bind _output_get_2 (Variables|Default|SetIsFindMoveRoute (or _outisfindmoveroute (Variables|Default|GetIsFindMoveRoute))))
            (if (not _output_get_2)
              (Utilities|Array|AppendArray (Variables|Default|GetRouteTaskManager) _outnextlocations)
              (bind _result (Math|Integer|IncrementInt (Variables|Default|GetNowTesk))
                (:%20%20
                  (Variables|Default|SetNowTesk _result)))
              (else
                (bind _result_2 (Math|Integer|IncrementInt (Variables|Default|GetNowTesk) :!label _label)
                  (:%20%20
                    (Variables|Default|SetNowTesk _result_2)))))
            (else
              (goto _label)))))
      ;[1 1 1] GreedyMap으로부터 findLocation(목적지) 에서 startLocation(출발지점)으로 오는 좌표값을 담은 Array 출력, 변수 RouteResults에 저장
      (Variables|Default|SetSerchingRoute (Variables|Default|GetFind%20Location))
      (bind _output_get_3 (Variables|Default|SetRouteResult (Utilities|Array|MakeArray)))
      (Utilities|Array|Clear _output_get_3)
      (while (and (not (and (== (.X (Utilities|Struct|BreakIntVector (Variables|Default|GetSerchingRoute))) (.X (Utilities|Struct|BreakIntVector (Variables|Default|GetPlayerLocation)))) (== (.Y (Utilities|Struct|BreakIntVector (Variables|Default|GetSerchingRoute))) (.Y (Utilities|Struct|BreakIntVector (Variables|Default|GetPlayerLocation)))))) (Utilities|Map|Contains (Variables|Default|GetGreedy%20Map) (Variables|Default|GetSerchingRoute)))
        (Utilities|Array|Add (Variables|Default|GetRouteResult) (.Value (Utilities|Map|Find (Variables|Default|GetGreedy%20Map) (Variables|Default|GetSerchingRoute))))
        (Variables|Default|SetSerchingRoute (Utilities|Struct|MakeIntVector (.X (Utilities|Struct|BreakIntVector (.Value (Utilities|Map|Find (Variables|Default|GetGreedy%20Map) (Variables|Default|GetSerchingRoute))))) (.Y (Utilities|Struct|BreakIntVector (.Value (Utilities|Map|Find (Variables|Default|GetGreedy%20Map) (Variables|Default|GetSerchingRoute))))))))
      (Utilities|Array|Reverse (Variables|Default|GetRouteResult))
      (Utilities|Array|Add (Variables|Default|GetRouteResult) (Variables|Default|GetFind%20Location))
      (Variables|Default|SetIsNeedMakeGreedMap false))))

(event Custom|setMoveLocation
  (params (InputIsNeedMakeGreedMap :type Boolean) (BlockActorLocations :type Array%20of%20Actor%20Object%20References))
  (Variables|Default|SetCalcBlockInfoMap (Variables|Default|GetBlock%20Info%20Map))
  (for _array_element BlockActorLocations
    (bind _intvector (CallFunction|VectorLocation2IntLocation (Transformation|GetActorLocation _array_element)))
    (Utilities|Map|Add (Variables|Default|GetCalcBlockInfoMap) _intvector false))
  (bind _output_get (Variables|Default|SetIsNeedMakeGreedMap InputIsNeedMakeGreedMap))
  (if _output_get
    (if (Variables|Default|GetIsMoveFinished)
      (bind _intvector_2 (CallFunction|VectorLocation2IntLocation (Transformation|GetActorLocation)))
      (Variables|Default|SetPlayerLocation _intvector_2)
      ;[1 1 1] reset 0
      (Utilities|Array|Clear (Variables|Default|GetRouteResult))
      (Utilities|Array|Clear (Variables|Default|GetRouteTaskManager))
      (Utilities|Map|Clear (Variables|Default|GetGreedy%20Map))
      (Variables|Default|SetNowTesk 0)
      (Variables|Default|SetRouteTaskManager (Utilities|Array|MakeArray _intvector_2))
      ;[1 1 1] \GreedyMap에PlayerLocation부터 MaxIteration의 거리까지의 정보 f(x) = MI - pL * dt/dx를 이동한 경로값 (n+1,m),(n,m+1),(n-1,m),(n,m-1)의 Key, (n,m,Iteration)의 Value 형태를 Map으로 저장
      (for _index (range 0 (Variables|Default|GetMax%20Iteration))
        (while (== (.Z (Utilities|Struct|BreakIntVector (Utilities|Array|Get(acopy) (Variables|Default|GetRouteTaskManager) (Variables|Default|GetNowTesk)))) _index)
          (bind (_outnextlocations _outismaxiterationover _outisfindmoveroute) (CallFunction|CheckRoute4 (Variables|Default|GetGreedy%20Map) (Variables|Default|GetCalcBlockInfoMap) (Utilities|Array|Get(acopy) (Variables|Default|GetRouteTaskManager) (Variables|Default|GetNowTesk)) (Variables|Default|GetFind%20Location) _index (Variables|Default|GetMax%20Iteration)))
          (if (not _outismaxiterationover)
            (bind _output_get_2 (Variables|Default|SetIsFindMoveRoute (or _outisfindmoveroute (Variables|Default|GetIsFindMoveRoute))))
            (if (not _output_get_2)
              (Utilities|Array|AppendArray (Variables|Default|GetRouteTaskManager) _outnextlocations)
              (bind _result (Math|Integer|IncrementInt (Variables|Default|GetNowTesk))
                (:%20%20
                  (Variables|Default|SetNowTesk _result)))
              (else
                (bind _result_2 (Math|Integer|IncrementInt (Variables|Default|GetNowTesk) :!label _label)
                  (:%20%20
                    (Variables|Default|SetNowTesk _result_2)))))
            (else
              (goto _label)))))
      ;[1 1 1] GreedyMap으로부터 findLocation(목적지) 에서 startLocation(출발지점)으로 오는 좌표값을 담은 Array 출력, 변수 RouteResults에 저장
      (Variables|Default|SetSerchingRoute (Variables|Default|GetFind%20Location))
      (bind _output_get_3 (Variables|Default|SetRouteResult (Utilities|Array|MakeArray)))
      (Utilities|Array|Clear _output_get_3)
      (while (and (not (and (== (.X (Utilities|Struct|BreakIntVector (Variables|Default|GetSerchingRoute))) (.X (Utilities|Struct|BreakIntVector (Variables|Default|GetPlayerLocation)))) (== (.Y (Utilities|Struct|BreakIntVector (Variables|Default|GetSerchingRoute))) (.Y (Utilities|Struct|BreakIntVector (Variables|Default|GetPlayerLocation)))))) (Utilities|Map|Contains (Variables|Default|GetGreedy%20Map) (Variables|Default|GetSerchingRoute)))
        (Utilities|Array|Add (Variables|Default|GetRouteResult) (.Value (Utilities|Map|Find (Variables|Default|GetGreedy%20Map) (Variables|Default|GetSerchingRoute))))
        (Variables|Default|SetSerchingRoute (Utilities|Struct|MakeIntVector (.X (Utilities|Struct|BreakIntVector (.Value (Utilities|Map|Find (Variables|Default|GetGreedy%20Map) (Variables|Default|GetSerchingRoute))))) (.Y (Utilities|Struct|BreakIntVector (.Value (Utilities|Map|Find (Variables|Default|GetGreedy%20Map) (Variables|Default|GetSerchingRoute))))))))
      (Utilities|Array|Reverse (Variables|Default|GetRouteResult))
      (Utilities|Array|Add (Variables|Default|GetRouteResult) (Variables|Default|GetFind%20Location))
      (Variables|Default|SetIsNeedMakeGreedMap false))))

(event EventBeginPlay
  (bind _asabp_player (Utilities|Casting|CastToABP_Player (Components|SkeletalMesh|GetAnimInstance (Variables|Default|GetSkeletalMesh))))
  (Variables|Default|SetAs%20ABP%20Player _asabp_player))

(event EventTick
  (params (DeltaSeconds :type Float%20%28single-precision%29)))

(fn ConstructionScript)

(fn Translate
  (params (GetToPointX :type Integer) (GetToPointY :type Integer))
  (bind _returnvalue (Transformation|GetActorLocation))
  (bind _returnvalue_2 (Transformation|GetActorLocation))
  (bind _returnvalue_3 (Transformation|GetActorLocation))
  (bind _returnvalue_4 (Math|Float|Floor (.x _returnvalue_3)))
  (bind _returnvalue_5 (Math|Vector|MakeVector (.x _returnvalue_2) (.y _returnvalue_2) 0.0))
  (LocalVariables|SetPointX (+ (* GetToPointX 100) 50))
  (LocalVariables|SetPointY (+ (* GetToPointY 100) 50))
  (Transformation|SetActorLocation (+ (Transformation|GetActorLocation) (* (Math|Vector|Normalize (- (Math|Vector|MakeVector (Math|Conversions|ToFloat(Integer) (LocalVariables|GetPointX)) (Math|Conversions|ToFloat(Integer) (LocalVariables|GetPointY)) 0.0) _returnvalue_5)) (Variables|Default|GetSpeed) (Utilities|Time|GetWorldDeltaSeconds))) false false)
  (Transformation|SetActorRotation (Math|Rotator|MakeRotator 0.0 0.0 (.Yaw (Math|Vector|GetYawPitchfromVector (Math|Vector|MakeVector (.x (- (Math|Vector|MakeVector (Math|Conversions|ToFloat(Integer) (LocalVariables|GetPointX)) (Math|Conversions|ToFloat(Integer) (LocalVariables|GetPointY)) 0.0) _returnvalue_5)) (.y (- (Math|Vector|MakeVector (Math|Conversions|ToFloat(Integer) (LocalVariables|GetPointX)) (Math|Conversions|ToFloat(Integer) (LocalVariables|GetPointY)) 0.0) _returnvalue_5)) 0.0)))))
  (if (>= (LocalVariables|GetPointX) 0)
    (LocalVariables|SetIsFinishX (and (<= (+ (LocalVariables|GetPointX) -5) _returnvalue_4) (<= _returnvalue_4 (+ (LocalVariables|GetPointX) 5))))
    (else
      (LocalVariables|SetIsFinishX (and (<= _returnvalue_4 (+ (LocalVariables|GetPointX) 5)) (<= (+ (LocalVariables|GetPointX) -5) _returnvalue_4)))))
  (if (>= (LocalVariables|GetPointY) 0)
    (LocalVariables|SetIsFinishY (and (<= (+ (LocalVariables|GetPointY) -5) (.y _returnvalue)) (<= (.y _returnvalue) (+ (LocalVariables|GetPointY) 5))))
    (else
      (LocalVariables|SetIsFinishY (and (<= (.y _returnvalue) (+ (LocalVariables|GetPointY) 5)) (<= (+ (LocalVariables|GetPointY) -5) (.y _returnvalue))))))
  (if (and (LocalVariables|GetIsFinishX) (LocalVariables|GetIsFinishY))
    (return (and (LocalVariables|GetIsFinishX) (LocalVariables|GetIsFinishY)))
    (else
      (return (and (LocalVariables|GetIsFinishX) (LocalVariables|GetIsFinishY))))))

(fn CheckRoute4
  (params (InGreedyMap :type Map%20of%20Int%20Vector%20Structures%20to%20Structs) (InBlockInfoMap :type Map%20of%20Int%20Vector%20Structures%20to%20Booleans) (InThisLocation :type Int%20Vector%20Structure) (InFindLocation :type Int%20Vector%20Structure) (InNowIteration :type Integer) (InMaxIteration :type Integer))
  (bind (_x _y) (Utilities|Struct|BreakIntVector InThisLocation))
  (bind (_x_2 _y_2) (Utilities|Struct|BreakIntVector InThisLocation))
  (bind (_x_3 _y_3) (Utilities|Struct|BreakIntVector InFindLocation))
  (bind (_x_4 _y_4) (Utilities|Struct|BreakIntVector InThisLocation))
  (bind (_x_5 _y_5) (Utilities|Struct|BreakIntVector InFindLocation))
  (bind (_x_6 _y_6) (Utilities|Struct|BreakIntVector InThisLocation))
  (bind (_x_7 _y_7) (Utilities|Struct|BreakIntVector InFindLocation))
  (bind (_x_8 _y_8) (Utilities|Struct|BreakIntVector InThisLocation))
  (bind (_x_9 _y_9) (Utilities|Struct|BreakIntVector InFindLocation))
  (bind (_x_10 _y_10) (Utilities|Struct|BreakIntVector InThisLocation))
  (bind (_x_11 _y_11) (Utilities|Struct|BreakIntVector InThisLocation))
  (bind (_x_12 _y_12) (Utilities|Struct|BreakIntVector InThisLocation))
  (bind _returnvalue (+ InNowIteration 1))
  (bind _returnvalue_2 (+ InNowIteration 1))
  (bind _returnvalue_3 (+ InNowIteration 1))
  (bind _returnvalue_4 (+ InNowIteration 1))
  (bind _returnvalue_5 (+ _y_11 -1))
  (bind _returnvalue_6 (+ _x 1))
  (bind _returnvalue_7 (+ _y_2 1))
  (bind _returnvalue_8 (+ _x_10 -1))
  (bind _intvector (Utilities|Struct|MakeIntVector _returnvalue_6 _y))
  (bind _intvector_2 (Utilities|Struct|MakeIntVector _x_2 _returnvalue_7))
  (bind _intvector_3 (Utilities|Struct|MakeIntVector _returnvalue_8 _y_10))
  (bind _intvector_4 (Utilities|Struct|MakeIntVector _x_11 _returnvalue_5))
  (LocalVariables|SetLocalNextLoopFindLocation (Utilities|Array|MakeArray))
  (LocalVariables|SetLocalMaxIteration InMaxIteration)
  (LocalVariables|SetLocalIsFindMoveRoute false)
  (Utilities|FlowControl|Sequence
    (:then_0
      (if (>= (LocalVariables|GetLocalMaxIteration) InNowIteration)
        (if (not (.ReturnValue (Utilities|Map|Find (Variables|Default|GetGreedy%20Map) _intvector)))
          (if (not (.ReturnValue (Utilities|Map|Find InBlockInfoMap _intvector)))
            (Utilities|Map|Add (Variables|Default|GetGreedy%20Map) _intvector (Utilities|Struct|MakeIntVector _x_4 _y_4 _returnvalue_2))
            (Utilities|Array|AppendArray (LocalVariables|GetLocalNextLoopFindLocation) (Utilities|Array|MakeArray (Utilities|Struct|MakeIntVector _returnvalue_6 _y _returnvalue_2)))
            (LocalVariables|SetLocalIsFindMoveRoute (and (== _returnvalue_6 _x_5) (== _y _y_5)))))
        (else
          (return (LocalVariables|GetLocalNextLoopFindLocation) true false))))
    (:then_1
      (if (>= (LocalVariables|GetLocalMaxIteration) InNowIteration)
        (if (not (.ReturnValue (Utilities|Map|Find (Variables|Default|GetGreedy%20Map) _intvector_2)))
          (if (not (.ReturnValue (Utilities|Map|Find InBlockInfoMap _intvector_2)))
            (Utilities|Map|Add (Variables|Default|GetGreedy%20Map) _intvector_2 (Utilities|Struct|MakeIntVector _x_6 _y_6 _returnvalue_3))
            (Utilities|Array|AppendArray (LocalVariables|GetLocalNextLoopFindLocation) (Utilities|Array|MakeArray (Utilities|Struct|MakeIntVector _x_2 _returnvalue_7 _returnvalue_3)))
            (LocalVariables|SetLocalIsFindMoveRoute (or (LocalVariables|GetLocalIsFindMoveRoute) (and (== _x_2 _x_7) (== _returnvalue_7 _y_7))))))
        (else
          (return (LocalVariables|GetLocalNextLoopFindLocation) true false))))
    (:then_2
      (if (>= (LocalVariables|GetLocalMaxIteration) InNowIteration)
        (if (not (Utilities|Map|Contains (Variables|Default|GetGreedy%20Map) _intvector_3))
          (if (not (.ReturnValue (Utilities|Map|Find InBlockInfoMap _intvector_3)))
            (Utilities|Map|Add (Variables|Default|GetGreedy%20Map) _intvector_3 (Utilities|Struct|MakeIntVector _x_8 _y_8 _returnvalue_4))
            (Utilities|Array|AppendArray (LocalVariables|GetLocalNextLoopFindLocation) (Utilities|Array|MakeArray (Utilities|Struct|MakeIntVector _returnvalue_8 _y_10 _returnvalue_4)))
            (LocalVariables|SetLocalIsFindMoveRoute (or (LocalVariables|GetLocalIsFindMoveRoute) (and (== _returnvalue_8 _x_9) (== _y_10 _y_9))))))
        (else
          (return (LocalVariables|GetLocalNextLoopFindLocation) true false))))
    (:then_3
      (if (>= (LocalVariables|GetLocalMaxIteration) InNowIteration)
        (if (not (.ReturnValue (Utilities|Map|Find (Variables|Default|GetGreedy%20Map) _intvector_4)))
          (if (not (.ReturnValue (Utilities|Map|Find InBlockInfoMap _intvector_4)))
            (Utilities|Map|Add (Variables|Default|GetGreedy%20Map) _intvector_4 (Utilities|Struct|MakeIntVector _x_12 _y_12 _returnvalue))
            (Utilities|Array|AppendArray (LocalVariables|GetLocalNextLoopFindLocation) (Utilities|Array|MakeArray (Utilities|Struct|MakeIntVector _x_11 _returnvalue_5 _returnvalue)))
            (LocalVariables|SetLocalIsFindMoveRoute (or (LocalVariables|GetLocalIsFindMoveRoute) (and (== _x_11 _x_3) (== _returnvalue_5 _y_3))))))
        (return (LocalVariables|GetLocalNextLoopFindLocation) false false)
        (else
          (return (LocalVariables|GetLocalNextLoopFindLocation) true false))))))

(fn CheckRoute8)

(fn AttackFocus
  (params (InTarget :type Actor%20Object%20Reference) (InCamera :type Actor%20Object%20Reference))
  (bind _asbp_camera_pawn (Utilities|Casting|CastToBP_CameraPawn InCamera)
    (:then
      (Default|CameraFocusActor _asbp_camera_pawn InTarget))
    (:CastFailed
      (Development|PrintString "BP_Player::AttackFocus CastFailed"))))

(fn Attack
  (params (Bullet :type Actor%20Object%20Reference) (AttackTarget :type Actor%20Object%20Reference))
  (bind _returnvalue (Transformation|GetActorLocation AttackTarget))
  (bind _arrow (Variables|Default|GetArrow))
  (bind _returnvalue_2 (Components|GetOwner _arrow))
  (bind _returnvalue_3 (Transformation|GetActorLocation _returnvalue_2))
  (bind _returnvalue_4 (- _returnvalue _returnvalue_3))
  (bind _returnvalue_5 (Game|SpawnActorfromClass "/Game/LSJ/BluePrint/BP_Bullet.BP_Bullet_C" (Math|Transform|MakeTransform _returnvalue_3 (Math|Rotator|MakeRotator 0.0 0.0 (.Yaw (Math|Vector|GetYawPitchfromVector (Math|Vector|MakeVector (.x _returnvalue_4) (.y _returnvalue_4) 0.0)))) "1.000000,1.000000,1.000000") "AlwaysSpawn" "MultiplyWithRoot" 0 0))
  (return _returnvalue_5 (Variables|/Game/LSJ/BluePrint/BP_Bullet.BP_Bullet_C|GetSpeed _returnvalue_5)))

(fn MakeGreedyMap
  (params (NewParam :type Map%20of%20Int%20Vector%20Structures%20to%20Structs) (NewParam1 :type Map%20of%20Int%20Vector%20Structures%20to%20Structs)))

(fn SelectEnemy
  (params (InPlayerLocation :type Int%20Vector%20Structure) (InEnemyLocation :type Int%20Vector%20Structure) (IgnoreCollisonOverlap :type Array%20of%20Actor%20Object%20References))
  (Development|ExecuteConsoleCommand "show splines" 0)
  (bind _vector (CallFunction|IntLocation2VectorLocation InPlayerLocation))
  (bind _vector_2 (CallFunction|IntLocation2VectorLocation InEnemyLocation))
  (bind _outhit (Collision|LineTraceByChannel (+ _vector "0.000000,0.000000,160.000000") (+ _vector_2 "0.000000,0.000000,160.000000") "TraceTypeQuery1" false IgnoreCollisonOverlap "None"))
  (return (not (.bblockinghit _outhit)) (Math|Vector|Distance(Vector) (.tracestart _outhit) (.traceend _outhit))))

(fn VectorLocation2IntLocation
  (params (Vector :type Vector))
  (bind _returnvalue (Math|Vector|MakeVector 0.01 0.01 0.0))
  (bind _returnvalue_2 (* Vector _returnvalue))
  (return (Utilities|Struct|MakeIntVector (Math|Float|Floor (.x _returnvalue_2)) (Math|Float|Floor (.y _returnvalue_2)))))

(fn IntLocation2VectorLocation
  (params (IntVector :type Int%20Vector%20Structure))
  (return (+ (* (Math|Conversions|ToVector(Float) IntVector) "100.000000,100.000000,0.000000") "50.000000,50.000000,0.000000")))

(fn SelectEnemy8
  (bind _vector (CallFunction|IntLocation2VectorLocation ""))
  (bind _vector_2 (CallFunction|IntLocation2VectorLocation ""))
  (bind _outhit (Collision|LineTraceByChannel (+ _vector "0.000000,0.000000,160.000000") (+ _vector_2 "0.000000,0.000000,160.000000") "TraceTypeQuery1" false 0 "None"))
  (return (not (.bblockinghit _outhit)) (Math|Vector|Distance(Vector) (.tracestart _outhit) (.traceend _outhit))))