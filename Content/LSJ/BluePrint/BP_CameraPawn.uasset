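; Player camera pawn that moves and turns from input and can jump to a cinematic view between two actors.
; Tick applies swept, yaw-relative movement and yaw rotation.
; CinematicViewActor2Actor saves the transform once, then takes the first supplied or default position with clear sight to HitActor, facing along the fire-to-hit yaw, else restores.
; ReturnPlayerCameraLocation restores that transform; FocusActor2Actor only saves it, while CameraFocusActor and CameraFollowActor are stubs.
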(event EventBeginPlay)

(event Collision|EventActorBeginOverlap
  (params (OtherActor :type Actor%20Object%20Reference)))

(event EventTick
  (params (DeltaSeconds :type Float%20%28single-precision%29))
  (bind _returnvalue (Transformation|GetActorRotation))
  (bind _returnvalue_2 (Input|AxisValues|GetCameraYaw))
  (bind _returnvalue_3 (+ (.yaw _returnvalue) _returnvalue_2))
  (bind _returnvalue_4 (Math|Conversions|ToVector(Float) _returnvalue_3))
  (bind _returnvalue_5 (Math|Vector|RotateVectorAroundAxis _returnvalue_4 (.yaw _returnvalue) "0.000000,0.000000,1.000000"))
  (Utilities|FlowControl|Sequence
    (:then_0
      ;[1 1 1] 카메라 방향키에 따른 이동
      (Transformation|SetActorLocation (+ (Transformation|GetActorLocation) (* (Math|Vector|RotateVector (Math|Vector|Normalize (Math|Vector|MakeVector (Input|AxisValues|GetVertical) (Input|AxisValues|GetHorizonal) 0.0)) (Variables|Default|Getyaw)) (Variables|Default|GetSpeed) (Utilities|Time|GetWorldDeltaSeconds))) true false))
    (:then_1
      ;[1 1 1] 카메라 qe키에 따른 회전이동
      (Variables|Default|Setyaw (Math|Rotator|MakeRotator 0.0 0.0 (.z _returnvalue_5)))
      (Transformation|SetActorRotation (Math|Rotator|MakeRotator (.roll _returnvalue) (.pitch _returnvalue) (.z _returnvalue_5))))))

(fn ConstructionScript)

(fn CinematicViewActor2Actor
  (params (FireActor :type Actor%20Object%20Reference) (HitActor :type Actor%20Object%20Reference) (overrideCameraPosition :type Array%20of%20Vectors))
  (bind _returnvalue (Transformation|GetActorLocation HitActor))
  (bind _returnvalue_2 (Transformation|GetActorLocation FireActor))
  (bind _self self)
  (bind _returnvalue_3 (- _returnvalue _returnvalue_2))
  (bind _returnvalue_4 (Math|Vector|Normalize _returnvalue_3))
  (LocalVariables|SetNewLocalVar overrideCameraPosition)
  (if (Variables|Default|GetSavedCameraLR)
    _
    (else
      (Variables|Default|SetCameraLocation (Transformation|GetActorLocation _self))
      (Variables|Default|SetCameraRotation (Transformation|GetActorRotation _self))))
  (Variables|Default|SetSavedCameraLR true)
  (if (Utilities|Array|IsNotEmpty (LocalVariables|GetNewLocalVar))
    _
    (else
      (Utilities|Array|AppendArray (LocalVariables|GetNewLocalVar) (Utilities|Array|MakeArray (+ _returnvalue_2 "-200.000000,200.000000,200.000000") (+ _returnvalue_2 "200.000000,200.000000,200.000000") (+ _returnvalue_2 "200.000000,-200.000000,400.000000")))))
  (bind _array_element (Utilities|Array|ForEachLoopwithBreak (LocalVariables|GetNewLocalVar))
    (:LoopBody
      (bind _outhit (Collision|LineTraceByChannel _array_element (+ _returnvalue "0.000000,0.000000,160.000000") "TraceTypeQuery1" false (Utilities|Array|MakeArray HitActor) "ForDuration"))
      (if (not (.bblockinghit _outhit))
        (Transformation|SetActorLocationAndRotation (.tracestart _outhit) (Math|Rotator|MakeRotator 0.0 0.0 (.Yaw (Math|Vector|GetYawPitchfromVector (Math|Vector|MakeVector (.x _returnvalue_4) (.y _returnvalue_4) 0.0)))))
        (Development|PrintString (Utilities|String|ToString(Vector) (.tracestart _outhit)))
        (return)))
    (:Completed
      (Transformation|SetActorLocationAndRotation (Variables|Default|GetCameraLocation) (Variables|Default|GetCameraRotation))
      (return))))

(fn ReturnPlayerCameraLocation
  (Transformation|SetActorLocationAndRotation (Variables|Default|GetCameraLocation) (Variables|Default|GetCameraRotation)))

(fn FocusActor2Actor
  (params (viewer :type Actor%20Object%20Reference) (selecter :type Actor%20Object%20Reference))
  (bind _self self)
  (if (Variables|Default|GetSavedCameraLR)
    _
    (else
      (Variables|Default|SetCameraLocation (Transformation|GetActorLocation _self))
      (Variables|Default|SetCameraRotation (Transformation|GetActorRotation _self))))
  (Variables|Default|SetSavedCameraLR true)
  (return))

(fn CameraFocusActor
  (params (Actor1 :type Actor%20Object%20Reference)))

(fn CameraFollowActor)