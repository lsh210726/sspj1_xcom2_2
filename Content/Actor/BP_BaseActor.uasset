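; BP_BaseActor is a base actor that glides horizontally toward the world origin every frame.
; Tick passes a hardcoded zero vector to ChangeActorLocation, which steps along the 2D direction to that target by Speed scaled with delta time.
; Movement teleports without sweeping, preserves height, and stops once X and Y are within a small tolerance of the target.
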(event EventBeginPlay)

(event Collision|EventActorBeginOverlap
  (params (OtherActor :type Actor%20Object%20Reference)))

(event EventTick
  (params (DeltaSeconds :type Float%20%28single-precision%29))
  (CallFunction|ChangeActorLocation "0, 0, 0"))

(fn ConstructionScript)

(fn ChangeActorLocation
  (params (targetLocation :type Vector))
  (bind (_x _y) (Math|Vector|BreakVector targetLocation))
  (bind _returnvalue (Transformation|GetActorLocation))
  (if (not (Utilities|Operators|EqualEqual (Math|Vector|MakeVector _x _y 0.0) (Math|Vector|MakeVector (.x _returnvalue) (.y _returnvalue) 0.0) 1e+01))
    (Transformation|SetActorLocation (+ (* (Class|KismetMathLibrary|VectorNormal2D (- targetLocation (Transformation|GetActorLocation)) 0.0001) (Variables|Default|GetSpeed) (Utilities|Time|GetWorldDeltaSeconds)) (Transformation|GetActorLocation)) false true)))