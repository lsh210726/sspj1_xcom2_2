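; BP_PathManager is an actor that builds a grid of BP_RoadTile actors and reports which tiles are overlapped.
; Shortly after BeginPlay, nested loops spawn the evenly spaced square grid from the world origin, storing each tile in RoadTileArray.
; Every Tick it scans that array and prints the name of each tile whose IsOverlap flag is set, with no further path logic.
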(event EventBeginPlay
  (Utilities|FlowControl|Delay 0.2)
  (for _index (range 0 10)
    (Variables|Default|SetiX (* _index 200))
    (for _index_2 (range 0 10)
      (Variables|Default|SetiY (* _index_2 200))
      (bind _returnvalue (Game|SpawnActorfromClass "/Game/Actor/BP_RoadTile.BP_RoadTile_C" (Math|Conversions|ToTransform(Vector) (Math|Vector|MakeVector (Math|Conversions|ToFloat(Integer) (Variables|Default|GetiX)) (Math|Conversions|ToFloat(Integer) (Variables|Default|GetiY)) 0.0)) "Undefined" "MultiplyWithRoot" 0 0))
      (Utilities|Array|Add (Variables|Default|GetroadTileArray) _returnvalue))))

(event Collision|EventActorBeginOverlap
  (params (OtherActor :type Actor%20Object%20Reference)))

(event EventTick
  (params (DeltaSeconds :type Float%20%28single-precision%29))
  (for _array_element (Variables|Default|GetroadTileArray)
    (if (Variables|/Game/Actor/BP_RoadTile.BP_RoadTile_C|GetisOverlap _array_element)
      (Development|PrintString (Utilities|GetDisplayName _array_element)))))

(fn ConstructionScript)