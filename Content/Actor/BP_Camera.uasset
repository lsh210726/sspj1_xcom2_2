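; Turn-based tactics camera actor that becomes the view target and opens by framing the player group, then the enemy group.
; Tick then follows the first-found player, allowing pan, rotate and zoom, or the first-found BP_CBaseActor on enemy turns.
; Attacks frame the attacker-target midpoint, and a death call overrides everything to close in on the body.
; Motion uses per-frame lerps, with spring arm length scaled by actor distances.
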(event EventBeginPlay
  (Input|EnableInput (Game|GetPlayerController 0))
  (Game|Player|SetViewTargetwithBlend (Game|GetPlayerController 0) self 0.0 "VTBlend_Linear" 0.0 false)
  (bind _outactors (Actor|GetAllActorsOfClass "/Game/LSJ/BluePrint/BP_Player.BP_Player_C"))
  (Variables|Default|SetFocusedActorArr _outactors)
  (bind _outactors_2 (Actor|GetAllActorsOfClass "/Game/Actor/CActor/BP_CBaseActor.BP_CBaseActor_C"))
  (Variables|Default|SetEnemyArr _outactors_2)
  (Variables|Default|SetOpening_player true)
  (Variables|Default|Setopening_enemy false)
  (Utilities|FlowControl|Delay 2.0)
  (Variables|Default|Setopening_enemy true)
  (Utilities|FlowControl|Delay 2.0)
  (Variables|Default|SetOpening_player false)
  (Variables|Default|Setopening_enemy false)
  (Variables|Default|SetDefaultRot (Transformation|GetActorRotation)))

(event EventTick
  (params (DeltaSeconds :type Float%20%28single-precision%29))
  (bind _springarm (Variables|Default|GetSpringArm))
  (if (Variables|Default|GetOpening_player)
    (if (Variables|Default|Getopening_enemy)
      (CallFunction|EnemyGroupFocusing)
      (else
        (CallFunction|PlayerGroupFocusing)))
    (elif (Variables|Default|GetisDead)
      (Variables|Default|SetPreLoc (Transformation|GetActorLocation))
      (Transformation|SetActorLocation (Math|Vector|Lerp(Vector) (Variables|Default|GetPreLoc) (Transformation|GetActorLocation (Variables|Default|GetDead%20Actor)) 0.1) false false)
      (Variables|/Script/Engine.SpringArmComponent|SetTargetArmLength (Variables|Default|GetSpringArm) (Math|Float|Lerp (Variables|/Script/Engine.SpringArmComponent|GetTargetArmLength (Variables|Default|GetSpringArm)) (Variables|Default|GetarmLengMin) 0.1))
      (else
        (bind _asbp_xcomgame_state_base (Utilities|Casting|CastToBP_XCOMGameStateBase (Game|GetGameState)))
        (if (Variables|/Game/Actor/CActor/BP_XCOMGameStateBase.BP_XCOMGameStateBase_C|GetisPlayerTurn _asbp_xcomgame_state_base)
          (if (Variables|Default|GetisPlayerInAttack)
            (bind _player_attack_target (Variables|Default|GetPlayer%20Attack%20Target)
              (:then
                (bind _player_cam_owner (Variables|Default|GetPlayer%20Cam%20Owner)
                  (:then
                    (Variables|Default|SetCamInput false)
                    (Transformation|SetActorRotation (Variables|Default|GetDefaultRot))
                    (Transformation|SetActorLocation (Math|Vector|Lerp(Vector) (Variables|Default|GetPreLoc) (/ (+ (Transformation|GetActorLocation _player_cam_owner) (Transformation|GetActorLocation _player_attack_target)) 2.0) 0.1) false false)
                    (Variables|/Script/Engine.SpringArmComponent|SetTargetArmLength (Variables|Default|GetSpringArm) (Math|Float|Lerp (Variables|/Script/Engine.SpringArmComponent|GetTargetArmLength (Variables|Default|GetSpringArm)) (Math|Float|Clamp(Float) (Transformation|GetDistanceTo (Variables|Default|GetPlayer%20Cam%20Owner) (Variables|Default|GetPlayer%20Attack%20Target)) (Variables|Default|GetarmLengMin) 2.5e+03) 0.1)))
                  (:else
                    (Development|PrintString "bp_camera : player cam owner is not valid"))))
              (:else
                (Development|PrintString "bp_camera : player attack target is not valid")))
            (else
              (Variables|Default|SetPreLoc (Transformation|GetActorLocation))
              (bind _returnvalue (Actor|GetActorOfClass "/Game/LSJ/BluePrint/BP_Player.BP_Player_C"))
              (if (Variables|Default|GetCamInput)
                (Transformation|SetActorLocation (+ (Transformation|GetActorLocation) (* (Math|Vector|Normalize (+ (* (Transformation|GetActorForwardVector) (Input|AxisValues|GetVertical)) (* (Transformation|GetActorRightVector) (Input|AxisValues|GetHorizonal)))) 15)) false false)
                (Transformation|SetActorRotation (Math|Transform|TransformRotation (Transformation|GetActorTransform) (Math|Rotator|MakeRotator 0.0 0.0 (Input|AxisValues|GetCameraYaw))))
                (Variables|/Script/Engine.SpringArmComponent|SetTargetArmLength _springarm (+ (Variables|/Script/Engine.SpringArmComponent|GetTargetArmLength _springarm) (Input|AxisValues|GetCameraLength)))
                (elif (> (Math|Vector|VectorLength (- (Variables|Default|GetPreLoc) (Transformation|GetActorLocation _returnvalue))) 0.01)
                  (Transformation|SetActorLocation (Math|Vector|Lerp(Vector) (Variables|Default|GetPreLoc) (Transformation|GetActorLocation _returnvalue) 0.1) false false)
                  (Variables|/Script/Engine.SpringArmComponent|SetTargetArmLength (Variables|Default|GetSpringArm) (Math|Float|Lerp (Variables|/Script/Engine.SpringArmComponent|GetTargetArmLength (Variables|Default|GetSpringArm)) (Variables|Default|GetarmLengMin) 0.1))
                  (else
                    (Variables|Default|SetCamInput true))))))
          (else
            (Variables|Default|SetCamInput false)
            (Transformation|SetActorRotation (Variables|Default|GetDefaultRot))
            (Variables|Default|SetPreLoc (Transformation|GetActorLocation))
            (bind _returnvalue_2 (Actor|GetActorOfClass "/Game/Actor/CActor/BP_CBaseActor.BP_CBaseActor_C"))
            (if (Variables|/Game/Actor/CActor/BP_CBaseActor.BP_CBaseActor_C|GetAttack _returnvalue_2)
              (Transformation|SetActorLocation (Math|Vector|Lerp(Vector) (Variables|Default|GetPreLoc) (/ (+ (Transformation|GetActorLocation _returnvalue_2) (Transformation|GetActorLocation (Variables|/Script/SSPJ1_XCOM2.BaseActor|Gettarget _returnvalue_2))) 2.0) 0.1) false false)
              (Variables|/Script/Engine.SpringArmComponent|SetTargetArmLength (Variables|Default|GetSpringArm) (Math|Float|Lerp (Variables|/Script/Engine.SpringArmComponent|GetTargetArmLength (Variables|Default|GetSpringArm)) (Math|Float|Clamp(Float) (Transformation|GetDistanceTo _returnvalue_2 (Variables|/Script/SSPJ1_XCOM2.BaseActor|Gettarget _returnvalue_2)) (Variables|Default|GetarmLengMin) 2.5e+03) 0.1))
              (else
                (Transformation|SetActorLocation (Math|Vector|Lerp(Vector) (Variables|Default|GetPreLoc) (Transformation|GetActorLocation _returnvalue_2) 0.1) false false)
                (Variables|/Script/Engine.SpringArmComponent|SetTargetArmLength (Variables|Default|GetSpringArm) (Math|Float|Lerp (Variables|/Script/Engine.SpringArmComponent|GetTargetArmLength (Variables|Default|GetSpringArm)) (Variables|Default|GetarmLengMin) 0.1))))))))))

(event Input|AxisEvents|InputAxisHorizonal
  (params (AxisValue :type Float%20%28single-precision%29)))

(fn ConstructionScript)

(fn EnemyGroupFocusing
  (bind _outactors (Actor|GetAllActorsOfClass "/Game/Actor/CActor/BP_CBaseActor.BP_CBaseActor_C"))
  (Variables|Default|SetEnemyArr _outactors)
  (Variables|Default|SetPreLoc (Transformation|GetActorLocation))
  (bind _returnvalue (Class|GameplayStatics|GetActorArrayAverageLocation (Variables|Default|GetEnemyArr)))
  (Variables|Default|SetTargetLoc _returnvalue)
  (Transformation|SetActorLocation (Math|Vector|Lerp(Vector) (Variables|Default|GetPreLoc) (Variables|Default|GetTargetLoc) 0.1) false false)
  (for (_array_element _array_index) (Variables|Default|GetEnemyArr)
    (Variables|Default|SetEnemy _array_element)
    (for _index (range (+ _array_index 1) (- (Utilities|Array|Length (Variables|Default|GetPlayerArr)) 1))
      (Utilities|Array|Add (Variables|Default|GetDistanceArr) (Transformation|GetDistanceTo (Variables|Default|GetPlayer) (Utilities|Array|Get(acopy) (Variables|Default|GetPlayerArr) _index)))))
  (Variables|/Script/Engine.SpringArmComponent|SetTargetArmLength (Variables|Default|GetSpringArm) (Math|Float|Clamp(Float) (.MaxValue (Math|Float|MaxOfFloatArray (Variables|Default|GetDistanceArr))) (Variables|Default|GetarmLengMin) 2.5e+03))
  (Utilities|Array|Clear (Variables|Default|GetDistanceArr)))

(fn PlayerGroupFocusing
  (bind _outactors (Actor|GetAllActorsOfClass "/Game/LSJ/BluePrint/BP_Player.BP_Player_C"))
  (Variables|Default|SetPlayerArr _outactors)
  (Variables|Default|SetPreLoc (Transformation|GetActorLocation))
  (bind _returnvalue (Class|GameplayStatics|GetActorArrayAverageLocation (Variables|Default|GetPlayerArr)))
  (Variables|Default|SetTargetLoc _returnvalue)
  (Transformation|SetActorLocation (Math|Vector|Lerp(Vector) (Variables|Default|GetPreLoc) (Variables|Default|GetTargetLoc) 0.1) false false)
  (for (_array_element _array_index) (Variables|Default|GetPlayerArr)
    (Variables|Default|SetPlayer _array_element)
    (for _index (range (+ _array_index 1) (- (Utilities|Array|Length (Variables|Default|GetPlayerArr)) 1))
      (Utilities|Array|Add (Variables|Default|GetDistanceArr) (Transformation|GetDistanceTo (Variables|Default|GetPlayer) (Utilities|Array|Get(acopy) (Variables|Default|GetPlayerArr) _index)))))
  (Variables|/Script/Engine.SpringArmComponent|SetTargetArmLength (Variables|Default|GetSpringArm) (Math|Float|Clamp(Float) (.MaxValue (Math|Float|MaxOfFloatArray (Variables|Default|GetDistanceArr))) (Variables|Default|GetarmLengMin) 2.5e+03))
  (Utilities|Array|Clear (Variables|Default|GetDistanceArr)))

(fn PlayerAttackCam
  (params (PlayerCamOwner :type BP%20Player%20Object%20Reference) (PlayerAttackTarget :type BP%20C%20Base%20Actor%20Object%20Reference))
  (Variables|Default|SetPlayer%20Cam%20Owner PlayerCamOwner)
  (Variables|Default|SetPlayer%20Attack%20Target PlayerAttackTarget)
  (Variables|Default|SetisPlayerInAttack true))

(fn PlayerAttackoverCam
  (Variables|Default|SetisPlayerInAttack false))

(fn SomeoneDead
  (params (DeadActor :type Actor%20Object%20Reference))
  (Variables|Default|SetDead%20Actor DeadActor)
  (Variables|Default|SetisDead true))