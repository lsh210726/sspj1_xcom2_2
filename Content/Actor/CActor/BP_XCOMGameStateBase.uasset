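; Game state for an XCOM-style turn-based game, managing player and enemy turns, mission flow, ambient sound and music.
; After a short delay, BeginPlay shows the enemy activity widget and starts the player turn.
; Turn setters animate that widget, set IsPlayerTurn and fire player or enemy dispatchers.
; ComputingHitEnemy always applies the attacker's default damage, leaving its accuracy roll unused, while missioncomplete stops music and shows completion and game-over widgets.
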(event Custom|PlayerTurnDispatcher_Event)

(event Custom|ComputingHitEnemy
  (params (AttackedEnemy :type BP%20C%20Base%20Actor%20Object%20Reference) (AttackerActor :type BP%20Player%20Object%20Reference))
  (Default|ApplyDamage AttackedEnemy (Variables|/Game/LSJ/BluePrint/BP_Player.BP_Player_C|GetDefaultDamage AttackerActor)))

(event Custom|mission%20complete
  (Audio|Components|Audio|Stop (Variables|Default|GetBGM))
  (Default|CheckboxCheck (Variables|Default|GetEnemyActivityWidget))
  (Utilities|FlowControl|Delay 5.0)
  (Default|MissionCompleteEvent (Variables|Default|GetEnemyActivityWidget))
  (bind _returnvalue (UserInterface|CreateWidget "/Game/Actor/widget/WB_GameOver.WB_GameOver_C"))
  (bind _output_get (Variables|Default|SetGameOverWidget _returnvalue))
  (UserInterface|Viewport|AddtoViewport _output_get 0)
  (Class|UserWidget|PlayAnimationForward (Variables|Default|GetGameOverWidget) (Variables|/Game/Actor/widget/WB_GameOver.WB_GameOver_C|GetmissionCompleteAnim (Variables|Default|GetGameOverWidget)) 1.0 false))

(event EventBeginPlay
  (bind _returnvalue (Audio|SpawnSound2D "/Game/Sound/onlymp3_to_-_Free_Sound_Effects_Nature_Sounds_Royalty_free_Non_Copyrighted_Sound_Effects_-FwVTkB-BIvM-192k-1706074621__mp3cut_net_.onlymp3_to_-_Free_Sound_Effects_Nature_Sounds_Royalty_free_Non_Copyrighted_Sound_Effects_-FwVTkB-BIvM-192k-1706074621__mp3cut_net_" 0.2 1.0 0.0 0))
  (Variables|Default|SetambientSound _returnvalue)
  (bind _returnvalue_2 (Audio|SpawnSound2D "/Game/Sound/Ambush-pLWLt2Tz_9c-192k-1706075699__online-audio-converter_com_.Ambush-pLWLt2Tz_9c-192k-1706075699__online-audio-converter_com_" 0.5 1.0 0.0 0))
  (Variables|Default|SetBGM _returnvalue_2)
  (Utilities|FlowControl|Delay 4.0)
  (bind _returnvalue_3 (UserInterface|CreateWidget "/Game/Actor/widget/WB_EnemyActivity.WB_EnemyActivity_C"))
  (bind _output_get (Variables|Default|SetEnemyActivityWidget _returnvalue_3))
  (UserInterface|Viewport|AddtoViewport _output_get 0)
  (CallFunction|SetPlayerTurnon)
  (Class|UserWidget|PlayAnimationForward (Variables|Default|GetEnemyActivityWidget) (Variables|/Game/Actor/widget/WB_EnemyActivity.WB_EnemyActivity_C|GetOBJStart (Variables|Default|GetEnemyActivityWidget)) 1.0 false))

(event EventTick
  (params (DeltaSeconds :type Float%20%28single-precision%29)))

(fn ConstructionScript)

(fn SetPlayerTurnon
  (bind _enemyactivitywidget (Variables|Default|GetEnemyActivityWidget))
  (Class|UserWidget|PlayAnimationReverse _enemyactivitywidget (Variables|/Game/Actor/widget/WB_EnemyActivity.WB_EnemyActivity_C|GetEnemyActivity _enemyactivitywidget) 1.0 false)
  (Variables|Default|SetisPlayerTurn true)
  (Default|CallPlayerTurnDispatcher))

(fn SetPlayerTurnOff
  (bind _enemyactivitywidget (Variables|Default|GetEnemyActivityWidget))
  (Class|UserWidget|PlayAnimationForward _enemyactivitywidget (Variables|/Game/Actor/widget/WB_EnemyActivity.WB_EnemyActivity_C|GetEnemyActivity _enemyactivitywidget) 1.0 false)
  (Variables|Default|SetisPlayerTurn false)
  (Default|CallEnemyTurnDispatcher))