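; Base enemy actor for an XCOM-style turn-based game, with HP, a widget health bar and a squash-flat death.
; On BeginPlay it binds its turn action to the game state's enemy-turn dispatcher.
; On its turn it moves to cover, then fires a debug-line attack trace at Target whose result is unused.
; Delay loops poll the Move and IsInAction flags before handing the turn back to the player.
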(event Custom|applyDamage
  (params (Damage :type Float%20%28double-precision%29))
  (if (> (Variables|Default|GetHP) 0.0)
    (bind _output_get (Variables|Default|SetHP (- (Variables|Default|GetHP) Damage)))
    (Variables|/Game/Actor/widget/AIHPBar.AIHPBar_C|SetWidgetBindHP (Variables|Default|GetAs%20AIHPBar) _output_get)
    (else
      (Development|PrintString "Enemy Dead" true false "(R=1.000000,G=0.000000,B=0.045011,A=1.000000)")
      (Transformation|SetActorScale3D "1.200000,1.200000,0.200000"))))

(event Custom|coverNAttack
  ;[1 0.8505 0.7157] 엄폐물로 이동 후 공격
  (Class|BaseActor|FindCoverNMove)
  (if (Variables|Default|Getmove) :!label _label
    (Utilities|FlowControl|Delay 0.2)
    (goto _label)
    (else
      (Rendering|Debug|DrawDebugLine (Transformation|GetActorLocation) (Transformation|GetActorLocation (Variables|Default|Gettarget)) "(R=1.000000,G=0.252688,B=0.000000,A=1.000000)" 1.0 11.0)
      (Transformation|SetActorScale3D "1.000000,1.000000,1.500000")
      (bind (_outhit _returnvalue) (Class|KismetSystemLibrary|LineTraceSinglebyProfile (Transformation|GetActorLocation) (Transformation|GetActorLocation (Variables|Default|Gettarget)) "Attack" false 0 "None" true))
      (if _returnvalue
        _
        (else
          _))
      (Utilities|Casting|CastToBP_Player (.HitActor (Collision|BreakHitResult _outhit))
        (:then
          _)
        (:CastFailed
          _))
      (Variables|Default|SetisInAction false)
      (Utilities|FlowControl|Delay 0.5)
      (Transformation|SetActorScale3D "1.000000,1.000000,1.000000"))))

(event Custom|enemyTurnAction
  (Development|PrintString "enemy turn!")
  (Variables|Default|SetisInAction true)
  (CallFunction|CoverNAttack)
  (if (Variables|Default|GetisInAction) :!label _label
    (Utilities|FlowControl|Delay 0.2)
    (goto _label)
    (else
      (Default|SetPlayerTurnon (Variables|Default|GetAs%20BP%20XCOMGame%20State%20Base)))))

(event EventBeginPlay
  (bind _asaihpbar (Utilities|Casting|CastToAIHPBar (UserInterface|GetUserWidgetObject (Variables|Default|GetHPBar))))
  (Variables|Default|SetAs%20AIHPBar _asaihpbar)
  (bind _asbp_xcomgame_state_base (Utilities|Casting|CastToBP_XCOMGameStateBase (Game|GetGameState)))
  (bind _output_get (Variables|Default|SetAs%20BP%20XCOMGame%20State%20Base _asbp_xcomgame_state_base))
  (EventDispatchers|BindEventtoEnemyTurnDispatcher _output_get (delegate Custom|enemyTurnAction)))

(event Collision|EventActorBeginOverlap
  (params (OtherActor :type Actor%20Object%20Reference)))

(event EventTick
  (params (DeltaSeconds :type Float%20%28single-precision%29)))

(fn ConstructionScript)